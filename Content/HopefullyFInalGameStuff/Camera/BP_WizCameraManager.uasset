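; Player camera manager that frames the wizard player together with the first pawn tagged "CamTarget".
; BeginPlay gathers the tagged pawns, and Tick measures the distance from the controlled pawn to the first.
; BlueprintUpdateCamera centers on their midpoint and pulls back along the player camera's forward vector by that distance, with a minimum but effectively no upper limit.
; Rotation and FOV come from the player's own camera component.
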(event EventBeginPlay
  (bind _outactors (Actor|GetAllActorsOfClasswithTag "/Script/Engine.Pawn" "CamTarget"))
  (bind _output_get (Variables|Default|SetCamTarget _outactors))
  (for (_ _array_index) _output_get
    _))

(event Collision|EventActorBeginOverlap
  (params (OtherActor :type Actor%20Object%20Reference)))

(event EventTick
  (params (DeltaSeconds :type Float%20%28single-precision%29))
  (Variables|Default|SetDistanceBetweenActors (Transformation|GetDistanceTo (Pawn|GetControlledPawn (Game|Player|GetOwningPlayerController)) (Utilities|Array|Get(acopy) (Variables|Default|GetCamTarget)))))

(fn ConstructionScript)

(fn BlueprintUpdateCamera
  (params (CameraTarget :type Actor%20Object%20Reference))
  (bind _distancebetweenactors (Variables|Default|GetDistanceBetweenActors))
  (bind _aswizard_protag_bp (Utilities|Casting|CastToWizardProtagBP CameraTarget))
  (bind _output_get (LocalVariables|SetPlayer _aswizard_protag_bp))
  (LocalVariables|SetMidpoint (/ (+ (Transformation|GetActorLocation (Utilities|Array|Get(acopy) (Variables|Default|GetCamTarget))) (Transformation|GetActorLocation (LocalVariables|GetPlayer))) 2.0))
  (LocalVariables|SetCamFov (Variables|/Script/Engine.CameraComponent|GetFieldOfView (Variables|/Script/WizardRush.WProtagWizard|GetCameraComp _output_get)))
  (bind _output_get_2 (Variables|Default|SetCamInitialRotation (.Rotation (Math|Transform|BreakTransform (Transformation|GetWorldTransform (Variables|/Script/WizardRush.WProtagWizard|GetCameraComp _output_get))))))
  (LocalVariables|SetCaminitialLocation (.Location (Math|Transform|BreakTransform (Transformation|GetWorldTransform (Variables|/Script/WizardRush.WProtagWizard|GetCameraComp _output_get)))))
  (return (+ (* (Math|Vector|GetForwardVector _output_get_2) (* (Math|Float|Clamp(Float) _distancebetweenactors 8e+02 _distancebetweenactors) -1.0)) (LocalVariables|GetMidpoint)) _output_get_2 (LocalVariables|GetCamFov) true))