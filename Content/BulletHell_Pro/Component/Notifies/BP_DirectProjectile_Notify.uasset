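; Anim notify that fires direct projectiles from a socket on the animated mesh, aimed along the owner's camera.
; On trigger, it checks the owner for an AC_BulletHell_Pro component and calls its SpawnDirectProjectile with the notify's projectile, spread, speed, homing, spin and spawn settings.
; It passes camera-forward start and end points, pushing the start out by the camera-to-socket distance.
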(fn ReceivedNotify
  (params (MeshComp :type Skeletal%20Mesh%20Component%20Object%20Reference) (Animation :type Anim%20Sequence%20Base%20Object%20Reference) (EventReference :type Anim%20Notify%20Event%20Reference%20Structure%20%28by%20ref%29))
  (bind _returnvalue (Components|GetOwner MeshComp))
  (bind _returnvalue_2 (Components|GetOwner MeshComp))
  (bind _in_socket_name (Variables|Default|GetIn%20Socket%20Name))
  (bind _returnvalue_3 (Actor|GetComponentbyClass _returnvalue "/Game/BulletHell_Pro/Component/AC_BulletHell_Pro.AC_BulletHell_Pro_C"))
  (bind _returnvalue_4 (Actor|GetComponentbyClass _returnvalue_2 "/Script/Engine.CameraComponent"))
  (bind _returnvalue_5 (Transformation|GetSocketLocation MeshComp _in_socket_name))
  (bind _returnvalue_6 (Transformation|GetWorldTransform _returnvalue_4))
  (Utilities|IsValid _returnvalue_3
    (:Is%20Valid
      (Default|SpawnDirectProjectile _returnvalue_3 (Variables|Default|GetSpawn%20Count) (|TraceStart (.location _returnvalue_6) (.rotation _returnvalue_6) _returnvalue_5) (|TraceEnd (.location _returnvalue_6) (.rotation _returnvalue_6) 3e+03) _returnvalue_5 (Variables|Default|GetProjectile) (Variables|Default|GetSpread%20Offset) (Variables|Default|GetProjectile%20Speed) (Variables|Default|GetIs%20Homing) (Variables|Default|GetIs%20Spinning) (Variables|Default|GetSpin%20Radius) (Variables|Default|GetSpawn%20Rate))
      (return false))
    (:Is%20Not%20Valid
      (return false))))