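; BP_EnemyBoss is an enemy boss character that shows an example of triggering a finisher attack on a nearby target.
; Each tick, while ACHitReaction reports it alive with no active action state, ACEnemyAI checks for a target in close range.
; A random roll then lets ACParrySystem fire a front-only finisher on that target.
; A graph comment places the QTE trigger in the finisher montage.
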(event EventBeginPlay
  (|CallParentFunction) ; This node is disabled and will not be called.\nDrag off pins to build functionality.
)

(event Collision|EventActorBeginOverlap
  (params (OtherActor :type Actor%20Object%20Reference)))

(event EventTick
  (params (DeltaSeconds :type Float%20%28single-precision%29))
  (bind _ac_hitreaction (Variables|Default|GetAC_HitReaction))
  (bind _ac_enemyai (Variables|Default|GetAC_EnemyAI))
  (bind (_returnvalue _targetactor) (Default|IsTargetinRange _ac_enemyai 0.0 3e+02))
  (|CallParentFunction DeltaSeconds)
  (if (Variables|/Game/CombatFury/UC_Assets/Components/HitReactionComponent/BluePrint/AC_HitReaction.AC_HitReaction_C|GetIsAlive _ac_hitreaction)
    ;[0.3469 0.01341 0] Finisher trigger example - QTE trigger can be found in the finisher montage. You should call similar function setup based on your game design doc.
    (switch Utilities|FlowControl|Switch|SwitchonE_ActionState (Default|GetActionState _ac_hitreaction)
      (:NewEnumerator0
        (if _returnvalue
          (if (== (Math|Random|RandomIntegerinRange 0 5) 1)
            (Default|FinisherEvent (Variables|Default|GetAC_ParrySystem) true _targetactor)))))))

(fn ConstructionScript
  (|CallParentFunction))