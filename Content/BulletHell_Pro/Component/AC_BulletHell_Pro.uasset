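; Bullet-hell component that spawns projectile patterns from its owner: direct, grid, arc, shockwave ring and homing peacock fan.
; Each pattern has an event that repeats its spawn function SpawnCount times, paced by the SpawnCounter delay macro.
; Spawn functions line trace to aim each projectile and pass it speed, homing, spin or snowfall settings.
; Direct shots add random spread, take the traced actor as homing target, and start at the socket unless AI-controlled.
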(fn CalculateMainDirection
  (params (StartLocation :type Vector) (EndLocation :type Vector) (Spread%20Offset :type Vector) (SocketLocation :type Vector))
  (bind _returnvalue (Components|GetOwner))
  (bind _returnvalue_2 (Components|GetOwner))
  (bind _returnvalue_3 (Transformation|GetActorForwardVector _returnvalue))
  (bind _returnvalue_4 (AI|GetAIController _returnvalue_2))
  (bind _returnvalue_5 (* _returnvalue_3 3e+01))
  (bind _returnvalue_6 (Utilities|IsValid _returnvalue_4))
  (bind _returnvalue_7 (+ SocketLocation _returnvalue_5))
  (bind _returnvalue_8 (select _returnvalue_6 StartLocation _returnvalue_7))
  (bind (_outhit _returnvalue_9) (Collision|LineTraceByChannel StartLocation EndLocation (Variables|Default|GetTrace%20Channel) false (Utilities|Array|MakeArray (Components|GetOwner)) (Variables|Default|GetDraw%20Debug%20Type) true (Variables|Default|GetTrace%20Color) (Variables|Default|GetTrace%20Hit%20Color) (Variables|Default|GetDraw%20Time)))
  (Variables|Default|SetHomingTarget (.HitActor (Collision|BreakHitResult _outhit)))
  (return (Math|Transform|MakeTransform _returnvalue_8 (Math|Rotator|FindLookatRotation _returnvalue_8 (Math|Vector|MakeVector (+ (.X (Math|Vector|BreakVector (Math|Vector|SelectVector (.ImpactPoint (Collision|BreakHitResult _outhit)) EndLocation _returnvalue_9))) (Math|Random|RandomFloatinRange (* (.x Spread%20Offset) -1.0) (.x Spread%20Offset))) (+ (.Y (Math|Vector|BreakVector (Math|Vector|SelectVector (.ImpactPoint (Collision|BreakHitResult _outhit)) EndLocation _returnvalue_9))) (Math|Random|RandomFloatinRange (* (.y Spread%20Offset) -1.0) (.y Spread%20Offset))) (+ (.Z (Math|Vector|BreakVector (Math|Vector|SelectVector (.ImpactPoint (Collision|BreakHitResult _outhit)) EndLocation _returnvalue_9))) (Math|Random|RandomFloatinRange (* (.z Spread%20Offset) -1.0) (.z Spread%20Offset))))))))

(fn SpawnShockwave
  (params (StartLocation :type Vector) (Projectile :type BP%20Base%20Projectile%20Class%20Reference) (Projectile%20H%20Sections :type Integer) (ProjectileSpeed :type Float%20%28double-precision%29) (AnglePitch :type Float%20%28double-precision%29) (AngleYaw :type Float%20%28double-precision%29) (Start%20Z%20Offset :type Float%20%28double-precision%29) (End%20Z%20Offset :type Float%20%28double-precision%29) (Velocity :type Vector) (IsSnowFall :type Boolean) (FreezDelay :type Float%20%28double-precision%29) (SnowFallDelay :type Float%20%28double-precision%29))
  (bind _returnvalue (+ StartLocation (Math|Vector|MakeVector 0.0 0.0 Start%20Z%20Offset)))
  (bind _returnvalue_2 (+ StartLocation (Math|Vector|MakeVector 0.0 0.0 Start%20Z%20Offset)))
  (for _index (range 0 Projectile%20H%20Sections)
    (bind (_outhit _returnvalue_3) (Collision|LineTraceByChannel _returnvalue_2 (+ _returnvalue_2 (* (Math|Vector|GetForwardVector (Math|Rotator|CombineRotators (Math|Rotator|MakeRotator 0.0 0.0 (* _index (/ 3.6e+02 (Math|Conversions|ToFloat(Integer) Projectile%20H%20Sections)))) (Math|Rotator|MakeRotator 0.0 AnglePitch AngleYaw))) 2e+03) (Math|Vector|MakeVector 0.0 0.0 End%20Z%20Offset)) "TraceTypeQuery1" false (Utilities|Array|MakeArray (Components|GetOwner)) (Variables|Default|GetDraw%20Debug%20Type) true (Variables|Default|GetTrace%20Color) (Variables|Default|GetTrace%20Hit%20Color) (Variables|Default|GetDraw%20Time)))
    (Game|SpawnActorfromClass Projectile (Math|Transform|MakeTransform _returnvalue (Math|Rotator|FindLookatRotation _returnvalue (Math|Vector|SelectVector (.ImpactPoint (Collision|BreakHitResult _outhit)) (+ _returnvalue_2 (* (Math|Vector|GetForwardVector (Math|Rotator|CombineRotators (Math|Rotator|MakeRotator 0.0 0.0 (* _index (/ 3.6e+02 (Math|Conversions|ToFloat(Integer) Projectile%20H%20Sections)))) (Math|Rotator|MakeRotator 0.0 AnglePitch AngleYaw))) 2e+03) (Math|Vector|MakeVector 0.0 0.0 End%20Z%20Offset)) _returnvalue_3))) "AlwaysSpawn" "SelectDefaultAtRuntime" (Components|GetOwner) 0 false ProjectileSpeed Velocity 0.0 false FreezDelay SnowFallDelay IsSnowFall (Variables|/Script/Engine.Actor|GetInstigator (Components|GetOwner)))))

(fn SpawnGrid
  (params (TraceStart :type Vector) (Projectile :type BP%20Base%20Projectile%20Class%20Reference) (Projectile%20H%20Sections :type Integer) (Projectile%20V%20Sections :type Integer) (ProjectileGap :type Float%20%28double-precision%29) (ProjectileSpeed :type Float%20%28double-precision%29) (TargetLocation :type Vector))
  (bind _returnvalue (Math|Rotator|FindLookatRotation TraceStart TargetLocation))
  (bind _returnvalue_2 (Math|Vector|GetRightVector _returnvalue))
  (for _index (range 1 Projectile%20V%20Sections)
    (for _index_2 (range 1 Projectile%20H%20Sections)
      (bind (_outhit _returnvalue_3) (Collision|LineTraceByChannel (+ (+ TraceStart (Math|Vector|MakeVector 0.0 0.0 (* _index ProjectileGap))) (+ (* _returnvalue_2 (* _index_2 ProjectileGap)) (* _returnvalue_2 (/ (* Projectile%20H%20Sections ProjectileGap) -2.0)) (* (Transformation|GetActorUpVector (Components|GetOwner)) (/ (* (+ Projectile%20V%20Sections 1) ProjectileGap) -2.0)))) (+ (+ (+ TraceStart (Math|Vector|MakeVector 0.0 0.0 (* _index ProjectileGap))) (+ (* _returnvalue_2 (* _index_2 ProjectileGap)) (* _returnvalue_2 (/ (* Projectile%20H%20Sections ProjectileGap) -2.0)) (* (Transformation|GetActorUpVector (Components|GetOwner)) (/ (* (+ Projectile%20V%20Sections 1) ProjectileGap) -2.0)))) (Math|Vector|GetForwardVector (Math|Rotator|FindLookatRotation TraceStart TargetLocation))) "TraceTypeQuery1" false 0 (Variables|Default|GetDraw%20Debug%20Type) true (Variables|Default|GetTrace%20Color) (Variables|Default|GetTrace%20Hit%20Color) (Variables|Default|GetDraw%20Time)))
      (Game|SpawnActorfromClass Projectile (Math|Transform|MakeTransform (+ (+ TraceStart (Math|Vector|MakeVector 0.0 0.0 (* _index ProjectileGap))) (+ (* _returnvalue_2 (* _index_2 ProjectileGap)) (* _returnvalue_2 (/ (* Projectile%20H%20Sections ProjectileGap) -2.0)) (* (Transformation|GetActorUpVector (Components|GetOwner)) (/ (* (+ Projectile%20V%20Sections 1) ProjectileGap) -2.0)))) (Math|Rotator|FindLookatRotation (+ (+ TraceStart (Math|Vector|MakeVector 0.0 0.0 (* _index ProjectileGap))) (+ (* _returnvalue_2 (* _index_2 ProjectileGap)) (* _returnvalue_2 (/ (* Projectile%20H%20Sections ProjectileGap) -2.0)) (* (Transformation|GetActorUpVector (Components|GetOwner)) (/ (* (+ Projectile%20V%20Sections 1) ProjectileGap) -2.0)))) (Math|Vector|SelectVector (.ImpactPoint (Collision|BreakHitResult _outhit)) (+ (+ (+ TraceStart (Math|Vector|MakeVector 0.0 0.0 (* _index ProjectileGap))) (+ (* _returnvalue_2 (* _index_2 ProjectileGap)) (* _returnvalue_2 (/ (* Projectile%20H%20Sections ProjectileGap) -2.0)) (* (Transformation|GetActorUpVector (Components|GetOwner)) (/ (* (+ Projectile%20V%20Sections 1) ProjectileGap) -2.0)))) (Math|Vector|GetForwardVector (Math|Rotator|FindLookatRotation TraceStart TargetLocation))) _returnvalue_3))) "AlwaysSpawn" "SelectDefaultAtRuntime" (Components|GetOwner) 0 false ProjectileSpeed "33.000000,0.000000,0.000000" 0.0 false 4.0 0.2 false (Variables|/Script/Engine.Actor|GetInstigator (Components|GetOwner))))))

(fn SpawnArc
  (params (TraceStart :type Vector) (Projectile :type BP%20Base%20Projectile%20Class%20Reference) (Projectile%20V%20Sections :type Integer) (Projectile%20H%20Sections :type Integer) (ProjectileGap :type Float%20%28double-precision%29) (ProjectileSpeed :type Float%20%28double-precision%29) (TargetLocation :type Vector))
  (bind _returnvalue (Math|Rotator|FindLookatRotation TraceStart TargetLocation))
  (bind _returnvalue_2 (Math|Vector|GetRightVector _returnvalue))
  (for _index (range 1 Projectile%20V%20Sections)
    (for _index_2 (range 1 Projectile%20H%20Sections)
      (bind (_outhit _returnvalue_3) (Collision|LineTraceByChannel TraceStart (+ TraceStart (Math|Vector|GetForwardVector (Math|Rotator|FindLookatRotation (+ TraceStart (Math|Vector|MakeVector 0.0 0.0 (* _index ProjectileGap)) (+ (* _returnvalue_2 (* _index_2 ProjectileGap)) (* _returnvalue_2 (/ (* Projectile%20H%20Sections ProjectileGap) -2.0)) (Math|Vector|MakeVector 0.0 0.0 (/ (* Projectile%20V%20Sections ProjectileGap) -2.0)))) TargetLocation))) "TraceTypeQuery1" false 0 (Variables|Default|GetDraw%20Debug%20Type) true (Variables|Default|GetTrace%20Color) (Variables|Default|GetTrace%20Hit%20Color) (Variables|Default|GetDraw%20Time)))
      (Game|SpawnActorfromClass Projectile (Math|Transform|MakeTransform TraceStart (Math|Rotator|FindLookatRotation TraceStart (Math|Vector|SelectVector (.ImpactPoint (Collision|BreakHitResult _outhit)) (+ TraceStart (Math|Vector|GetForwardVector (Math|Rotator|FindLookatRotation (+ TraceStart (Math|Vector|MakeVector 0.0 0.0 (* _index ProjectileGap)) (+ (* _returnvalue_2 (* _index_2 ProjectileGap)) (* _returnvalue_2 (/ (* Projectile%20H%20Sections ProjectileGap) -2.0)) (Math|Vector|MakeVector 0.0 0.0 (/ (* Projectile%20V%20Sections ProjectileGap) -2.0)))) TargetLocation))) _returnvalue_3))) "AlwaysSpawn" "SelectDefaultAtRuntime" (Components|GetOwner) 0 false ProjectileSpeed "33.000000,0.000000,0.000000" 0.0 false 4.0 0.2 false (Variables|/Script/Engine.Actor|GetInstigator (Components|GetOwner))))))

(fn SpawnDirect
  (params (StartLocation :type Vector) (EndLocation :type Vector) (SocketLocation :type Vector) (Projectile :type BP%20Base%20Projectile%20Class%20Reference) (Spread%20Offset :type Vector) (ProjectileSpeed :type Float%20%28double-precision%29) (IsHoming :type Boolean) (IsSpinning :type Boolean) (SpinRadius :type Float%20%28double-precision%29))
  (bind _transform (CallFunction|CalculateMainDirection StartLocation EndLocation Spread%20Offset SocketLocation))
  (Game|SpawnActorfromClass Projectile _transform "AlwaysSpawn" "SelectDefaultAtRuntime" (Components|GetOwner) (Variables|Default|GetHomingTarget) IsHoming ProjectileSpeed "33.000000,0.000000,0.000000" SpinRadius IsSpinning 4.0 0.2 false (Variables|/Script/Engine.Actor|GetInstigator (Components|GetOwner))))

(fn Spawnpeacock
  (params (StartLocation :type Vector) (Projectile :type BP%20Base%20Projectile%20Class%20Reference) (ProjectileSpeed :type Float%20%28double-precision%29) (Projectile%20Sections :type Integer) (ProjectileSpread :type Float%20%28double-precision%29) (AngleDirection :type Float%20%28double-precision%29) (Projectile%20Pitch :type Float%20%28double-precision%29) (Projectile%20Yaw :type Float%20%28double-precision%29) (Start%20Z%20Offset :type Float%20%28double-precision%29) (HomingTarget :type Actor%20Object%20Reference))
  (bind _returnvalue (+ StartLocation (Math|Vector|MakeVector 0.0 0.0 Start%20Z%20Offset)))
  (bind _returnvalue_2 (+ StartLocation (Math|Vector|MakeVector 0.0 0.0 Start%20Z%20Offset)))
  (for _index (range 0 Projectile%20Sections)
    (bind (_outhit _returnvalue_3) (Collision|LineTraceByChannel _returnvalue_2 (+ _returnvalue_2 (* (Math|Vector|GetForwardVector (Math|Rotator|CombineRotators (Math|Rotator|MakeRotator 0.0 0.0 (* _index (/ AngleDirection (Math|Conversions|ToFloat(Integer) Projectile%20Sections)))) (Math|Rotator|MakeRotator 0.0 Projectile%20Pitch Projectile%20Yaw))) ProjectileSpread) (* (Transformation|GetActorForwardVector (Components|GetOwner)) 2.5e+03)) "TraceTypeQuery1" false (Utilities|Array|MakeArray (Components|GetOwner)) (Variables|Default|GetDraw%20Debug%20Type) true (Variables|Default|GetTrace%20Color) (Variables|Default|GetTrace%20Hit%20Color) (Variables|Default|GetDraw%20Time)))
    (Game|SpawnActorfromClass Projectile (Math|Transform|MakeTransform _returnvalue (Math|Rotator|FindLookatRotation _returnvalue (Math|Vector|SelectVector (.ImpactPoint (Collision|BreakHitResult _outhit)) (+ _returnvalue_2 (* (Math|Vector|GetForwardVector (Math|Rotator|CombineRotators (Math|Rotator|MakeRotator 0.0 0.0 (* _index (/ AngleDirection (Math|Conversions|ToFloat(Integer) Projectile%20Sections)))) (Math|Rotator|MakeRotator 0.0 Projectile%20Pitch Projectile%20Yaw))) ProjectileSpread) (* (Transformation|GetActorForwardVector (Components|GetOwner)) 2.5e+03)) _returnvalue_3))) "AlwaysSpawn" "SelectDefaultAtRuntime" (Components|GetOwner) HomingTarget true ProjectileSpeed "1.000000,0.000000,0.000000" 0.0 false 4.0 0.2 false (Variables|/Script/Engine.Actor|GetInstigator (Components|GetOwner)))))

(event Custom|Spawn%20Direct%20Projectile
  (params (SpawnCount :type Integer) (StartLocation :type Vector) (EndLocation :type Vector) (SocketLocation :type Vector) (Projectile :type BP%20Base%20Projectile%20Class%20Reference) (Spread%20Offset :type Vector) (ProjectileSpeed :type Float%20%28double-precision%29) (IsHoming :type Boolean) (IsSpinning :type Boolean) (SpinRadius :type Float%20%28double-precision%29) (Spawn%20Rate :type Float%20%28double-precision%29))
  (bind _output_get (Variables|Default|SetSpawnCount SpawnCount))
  (Math|Integer|DecrementInt _output_get
    (:%20%20
      (CallFunction|SpawnDirect StartLocation EndLocation SocketLocation Projectile Spread%20Offset ProjectileSpeed IsHoming IsSpinning SpinRadius :!label _label)
      (Utilities|SpawnCounter Spawn%20Rate
        (:%20%20
          (goto _label))))))

(event Custom|Spawn%20Grid%20Projectile
  (params (SpawnCount :type Integer) (SpawnRate :type Float%20%28double-precision%29) (Start :type Vector) (Projectile :type BP%20Base%20Projectile%20Class%20Reference) (Projectile%20H%20Sections :type Integer) (Projectile%20V%20Sections :type Integer) (ProjectileGap :type Float%20%28double-precision%29) (ProjectileSpeed :type Float%20%28double-precision%29) (Target :type Actor%20Object%20Reference))
  (bind _output_get (Variables|Default|SetSpawnCount SpawnCount))
  (Math|Integer|DecrementInt _output_get
    (:%20%20
      (CallFunction|SpawnGrid Start Projectile Projectile%20H%20Sections Projectile%20V%20Sections ProjectileGap ProjectileSpeed (Transformation|GetActorLocation Target) :!label _label)
      (Utilities|SpawnCounter SpawnRate
        (:%20%20
          (goto _label))))))

(event Custom|Spawn%20Arc%20Projectile
  (params (SpawnCount :type Integer) (Spawn%20Rate :type Float%20%28double-precision%29) (Start :type Vector) (Projectile :type BP%20Base%20Projectile%20Class%20Reference) (Projectile%20V%20Sections :type Integer) (Projectile%20H%20Sections :type Integer) (ProjectileGap :type Float%20%28double-precision%29) (ProjectileSpeed :type Float%20%28double-precision%29) (Target :type Actor%20Object%20Reference))
  (bind _output_get (Variables|Default|SetSpawnCount SpawnCount))
  (Math|Integer|DecrementInt _output_get
    (:%20%20
      (CallFunction|SpawnArc Start Projectile Projectile%20V%20Sections Projectile%20H%20Sections ProjectileGap ProjectileSpeed (Transformation|GetActorLocation Target) :!label _label)
      (Utilities|SpawnCounter Spawn%20Rate
        (:%20%20
          (goto _label))))))

(event Custom|Spawn%20Shockwave%20Projectile
  (params (SpawnCount :type Integer) (SpawnRate :type Float%20%28double-precision%29) (StartLocation :type Vector) (Projectile :type BP%20Base%20Projectile%20Class%20Reference) (ProjectileSections :type Integer) (ProjectileSpeed :type Float%20%28double-precision%29) (Projectile%20Pitch :type Float%20%28double-precision%29) (Projectile%20Yaw :type Float%20%28double-precision%29) (Start%20Z%20Offset :type Float%20%28double-precision%29) (End%20Z%20Offset :type Float%20%28double-precision%29) (IsSnowFall :type Boolean) (SnowFallDelay :type Float%20%28double-precision%29))
  (bind _output_get (Variables|Default|SetSpawnCount SpawnCount))
  (Math|Integer|DecrementInt _output_get
    (:%20%20
      (CallFunction|SpawnShockwave StartLocation Projectile ProjectileSections ProjectileSpeed Projectile%20Pitch Projectile%20Yaw Start%20Z%20Offset End%20Z%20Offset (Math|Vector|MakeVector 33.0 (Math|Conversions|ToFloat(Integer) (Variables|Default|GetSpawnCount)) 0.0) IsSnowFall (+ (Math|Conversions|ToFloat(Integer) (Variables|Default|GetSpawnCount)) SpawnRate) SnowFallDelay :!label _label)
      (Utilities|SpawnCounter SpawnRate
        (:%20%20
          (goto _label))))))

(event Custom|Spawn%20Peacock%20Projectile
  (params (SpawnCount :type Integer) (SpawnRate :type Float%20%28double-precision%29) (StartLocation :type Vector) (Projectile :type BP%20Base%20Projectile%20Class%20Reference) (ProjectileSpeed :type Float%20%28double-precision%29) (Projectile%20H%20Sections :type Integer) (ProjectileSpread :type Float%20%28double-precision%29) (AngleDirection :type Float%20%28double-precision%29) (Projectile%20Pitch :type Float%20%28double-precision%29) (Projectile%20Yaw :type Float%20%28double-precision%29) (Start%20Z%20Offset :type Float%20%28double-precision%29) (HomingTarget :type Actor%20Object%20Reference))
  (bind _output_get (Variables|Default|SetSpawnCount SpawnCount))
  (Math|Integer|DecrementInt _output_get
    (:%20%20
      (CallFunction|Spawnpeacock StartLocation Projectile ProjectileSpeed Projectile%20H%20Sections ProjectileSpread AngleDirection Projectile%20Pitch Projectile%20Yaw Start%20Z%20Offset HomingTarget :!label _label)
      (Utilities|SpawnCounter SpawnRate
        (:%20%20
          (goto _label))))))