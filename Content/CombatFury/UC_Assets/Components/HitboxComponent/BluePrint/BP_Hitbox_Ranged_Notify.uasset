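; Animation notify state that drives ranged attack hitboxes during a montage or animation by messaging the owner's AC_Hitbox component.
; Projectile attacks send the begin-trace message once at notify begin, while AOE and spell attacks resend it every tick.
; Each message carries the attack type, state and AOE, projectile and spell settings, and notify end always sends the end-trace message.
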(fn GetNotifyName
  (return "Hitbox Ranged Notify"))

(fn ReceivedNotifyEnd
  (params (MeshComp :type Skeletal%20Mesh%20Component%20Object%20Reference) (Animation :type Anim%20Sequence%20Base%20Object%20Reference) (EventReference :type Anim%20Notify%20Event%20Reference%20Structure%20%28by%20ref%29))
  (Class|BIHitbox|EndAttackTrace(Message) (Actor|GetComponentbyClass (Components|GetOwner MeshComp) "/Game/CombatFury/UC_Assets/Components/HitboxComponent/BluePrint/AC_Hitbox.AC_Hitbox_C"))
  (return false))

(fn ReceivedNotifyTick
  (params (MeshComp :type Skeletal%20Mesh%20Component%20Object%20Reference) (Animation :type Anim%20Sequence%20Base%20Object%20Reference) (FrameDeltaTime :type Float%20%28single-precision%29) (EventReference :type Anim%20Notify%20Event%20Reference%20Structure%20%28by%20ref%29))
  (switch Utilities|FlowControl|Switch|SwitchonE_Ranged_Attack_Type (Variables|Default|GetAttack%20Type)
    (:NewEnumerator1
      _)
    (:NewEnumerator4
      _))
  (Class|BIHitbox|BeginRangedAttackTrace(Message) (Actor|GetComponentbyClass (Components|GetOwner MeshComp) "/Game/CombatFury/UC_Assets/Components/HitboxComponent/BluePrint/AC_Hitbox.AC_Hitbox_C") (Variables|Default|GetAttack%20Type) (Variables|Default|GetAttack%20State) (Variables|Default|GetAOE%20Setting) (Variables|Default|GetProjectile%20Setting) (Variables|Default|GetSpell%20Setting))
  (return false))

(fn ReceivedNotifyBegin
  (params (MeshComp :type Skeletal%20Mesh%20Component%20Object%20Reference) (Animation :type Anim%20Sequence%20Base%20Object%20Reference) (TotalDuration :type Float%20%28single-precision%29) (EventReference :type Anim%20Notify%20Event%20Reference%20Structure%20%28by%20ref%29))
  (switch Utilities|FlowControl|Switch|SwitchonE_Ranged_Attack_Type (Variables|Default|GetAttack%20Type)
    (:NewEnumerator3
      (Class|BIHitbox|BeginRangedAttackTrace(Message) (Actor|GetComponentbyClass (Components|GetOwner MeshComp) "/Game/CombatFury/UC_Assets/Components/HitboxComponent/BluePrint/AC_Hitbox.AC_Hitbox_C") (Variables|Default|GetAttack%20Type) (Variables|Default|GetAttack%20State) (Variables|Default|GetAOE%20Setting) (Variables|Default|GetProjectile%20Setting) (Variables|Default|GetSpell%20Setting))
      (return false))))