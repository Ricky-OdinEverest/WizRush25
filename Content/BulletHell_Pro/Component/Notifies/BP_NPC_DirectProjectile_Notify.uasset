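; Animation notify that makes an NPC fire direct projectiles at the player during an animation.
; It finds the AC_BulletHell_Pro component on the mesh owner and calls SpawnDirectProjectile, doing nothing if the component is absent.
; Shots start at a named mesh socket and aim at the player pawn's current location.
; Notify variables set projectile class, count, spread, speed, spawn rate, homing and spin.
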(fn ReceivedNotify
  (params (MeshComp :type Skeletal%20Mesh%20Component%20Object%20Reference) (Animation :type Anim%20Sequence%20Base%20Object%20Reference) (EventReference :type Anim%20Notify%20Event%20Reference%20Structure%20%28by%20ref%29))
  (bind _returnvalue (Components|GetOwner MeshComp))
  (bind _returnvalue_2 (Actor|GetComponentbyClass _returnvalue "/Game/BulletHell_Pro/Component/AC_BulletHell_Pro.AC_BulletHell_Pro_C"))
  (Utilities|IsValid _returnvalue_2
    (:Is%20Valid
      (Default|SpawnDirectProjectile _returnvalue_2 (Variables|Default|GetSpawn%20Count) (Transformation|GetSocketLocation MeshComp (Variables|Default|GetIn%20Socket%20Name)) (Transformation|GetActorLocation (Game|Player|GetPlayerPawn 0)) "0, 0, 0" (Variables|Default|GetProjectile) (Variables|Default|GetSpread%20Offset) (Variables|Default|GetProjectile%20Speed) (Variables|Default|GetIs%20Homing) (Variables|Default|GetIs%20Spinning) (Variables|Default|GetSpin%20Radius) (Variables|Default|GetSpawn%20Rate))
      (return false))
    (:Is%20Not%20Valid
      (return false))))