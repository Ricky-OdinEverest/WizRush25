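; BP_Dummy is a combat training dummy character for the demo room, used with the parry and hit reaction components.
; On BeginPlay it copies its CanBeFinished flag to the parry system and, when set, lowers Health so it can be finished.
; If CanAttack is set, it replays an attack montage in a delayed loop spaced by the montage length, for as long as it is alive.
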(event EventBeginPlay
  (|CallParentFunction)
  ;[1 1 1] For demo room only
  (bind _output_get (Variables|/Game/CombatFury/UC_Assets/Components/ParryComponent/AC_ParryAttack.AC_ParryAttack_C|SetCanBeFinished (Variables|Default|GetAC_ParrySystem) (Variables|Default|GetCan%20be%20Finished)))
  (if _output_get
    (Variables|/Game/CombatFury/UC_Assets/Components/HitReactionComponent/BluePrint/AC_HitReaction.AC_HitReaction_C|SetHealth (Variables|Default|GetAC_HitReaction) 3e+01))
  (if (Variables|Default|GetCanAttack)
    (bind _returnvalue (Animation|Montage|MontagePlay (Components|SkeletalMesh|GetAnimInstance (Variables|Character|GetMesh)) (Variables|Default|GetMontage%20to%20Play) 1.0 "MontageLength" 0.0 true :!label _label))
    (if (Variables|/Game/CombatFury/UC_Assets/Components/HitReactionComponent/BluePrint/AC_HitReaction.AC_HitReaction_C|GetIsAlive (Variables|Default|GetAC_HitReaction))
      (Utilities|FlowControl|Delay (* _returnvalue 2.0))
      (goto _label))))

(event Collision|EventActorBeginOverlap
  (params (OtherActor :type Actor%20Object%20Reference)))

(fn ConstructionScript
  (|CallParentFunction))