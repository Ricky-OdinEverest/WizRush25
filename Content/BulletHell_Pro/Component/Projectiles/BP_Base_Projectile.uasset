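; Base projectile actor for a bullet hell game that damages what it hits, spawns impact VFX and sound, then destroys itself.
; Construction script sets velocity and speed, while BeginPlay configures optional homing on a Character target and an optional freeze-then-fall snowfall effect.
; A looping timer runs a sphere trace for hit detection, replacing Hit events that proved unreliable with spinning, and drives the optional sine/cosine spin offset.
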(event Custom|Hit%20Event
  (params (Hit :type Hit%20Result%20Structure%20%28by%20ref%29))
  (bind (_bblockinghit _binitialoverlap _time _distance _location _impactpoint _normal _impactnormal _physmat _hitactor) (Collision|BreakHitResult Hit))
  ;[1 1 1] On Hit Event, add your SFX
  (Effects|SpawnEmitteratLocation (Variables|Default|GetHit%20VFX) _location (Math|Rotator|MakeRotfromX _impactnormal) "2.000000,2.000000,2.000000")
  (Audio|SpawnSoundatLocation 0 _location "0, 0, 0" 1.0 1.0 0.0 0 0)
  (Game|Damage|ApplyDamage _hitactor (Variables|Default|GetBase%20Damage) 0 self)
  (Actor|DestroyActor))

(event Custom|Hit%20Detection%20Event
  (bind _returnvalue (Utilities|Time|GetTimeSeconds))
  (bind _spinradius (Variables|Default|GetSpinRadius))
  (bind _sphere (Variables|Default|GetSphere))
  (bind _returnvalue_2 (Transformation|GetWorldLocation _sphere))
  (bind _returnvalue_3 (* _returnvalue 1e+01))
  (Utilities|FlowControl|Sequence
    (:then_0
      ;[1 1 1] For some reason when added spinning motion, characters don't receive a hit while on idle. I had to come up with this custom detection to make it work. If you don't need a spinning projectile feel free to remove this section and use On hit event for the Sphere.
      (bind (_outhit _returnvalue_4) (Collision|SphereTraceByChannel _returnvalue_2 _returnvalue_2 (Variables|/Script/Engine.SphereComponent|GetSphereRadius (Variables|Default|GetSphere)) (Variables|Default|GetHit%20Trace%20Channel) false 0 "None"))
      (if _returnvalue_4
        (Utilities|FlowControl|DoOnce false
          (:Completed
            (CallFunction|HitEvent _outhit)))))
    (:then_1
      ;;[1 0.1885 0] Spinning motion
      (if (Variables|Default|GetIsSpinning)
        (bind _sphere_2 (Variables|Default|GetSphere)
          (:then
            (Transformation|SetRelativeLocation _sphere_2 (Math|Vector|MakeVector 0.0 (* (Math|Trig|Sin(Radians) _returnvalue_3) _spinradius) (* (Math|Trig|Cos(Radians) _returnvalue_3) _spinradius)) false false))
          (:else))))))

(event EventBeginPlay
  (bind _freezprojctile (Variables|Default|GetFreezProjctile))
  (Utilities|FlowControl|Sequence
    (:then_0
      (|HomingMechanics))
    (:then_1
      ;[1 1 1] Snow Fall Effect
      (if (Variables|Default|GetIsSnowFall)
        (Utilities|FlowControl|Sequence
          (:then_0
            (Utilities|FlowControl|Delay _freezprojctile)
            (Variables|Default|GetSphere
              (:then
                (Variables|/Script/Engine.MovementComponent|SetVelocity (Variables|Default|GetProjectileMovement) "0, 0, 0"))
              (:else)))
          (:then_1
            (Utilities|FlowControl|Delay (+ (/ _freezprojctile 2.0) (Variables|Default|GetSnowFallDelay)))
            (Variables|Default|GetSphere
              (:then
                (Variables|/Script/Engine.ProjectileMovementComponent|SetProjectileGravityScale (Variables|Default|GetProjectileMovement) 5.0))
              (:else))))))
    (:then_2
      (bind _returnvalue (Utilities|Time|SetTimerbyEvent (delegate Custom|Hit%20Detection%20Event) 0.01 true))
      (Variables|Default|SetHitTimer _returnvalue))))

(event EventDestroyed
  ;[1 1 1] Clear hit detection timer
  (Utilities|Time|ClearandInvalidateTimerbyHandle (Variables|Default|GetHitTimer)))

(fn ConstructionScript
  (bind _projectilemovement (Variables|Default|GetProjectileMovement))
  (Variables|/Script/Engine.MovementComponent|SetVelocity (Variables|Default|GetProjectileMovement) (Variables|Default|GetVelocity))
  (bind _output_get (Variables|/Script/Engine.ProjectileMovementComponent|SetInitialSpeed _projectilemovement (Variables|Default|GetProjectileSpeed)))
  (Variables|/Script/Engine.ProjectileMovementComponent|SetMaxSpeed _projectilemovement _output_get))