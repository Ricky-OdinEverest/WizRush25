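; MagicProjectileBP is the player's magic projectile, which damages what it hits.
; On spawn it plays a firing sound and makes its collision sphere ignore the instigator when moving.
; On hitting anything other than the instigator, it spawns a particle burst, applies point damage with the instigator as damage causer, then destroys itself.
; Debug sphere and damage print nodes are present but never run.
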(event OnComponentHit(SphereComp)
  (params (HitComponent :type Primitive%20Component%20Object%20Reference) (OtherActor :type Actor%20Object%20Reference) (OtherComp :type Primitive%20Component%20Object%20Reference) (NormalImpulse :type Vector :default "0, 0, 0") (Hit :type Hit%20Result%20Structure%20%28by%20ref%29))
  (bind (_bblockinghit _binitialoverlap _time _distance _location _impactpoint _normal _impactnormal _physmat _hitactor _hitcomponent _hitbonename _bonename _hititem _elementindex _faceindex _tracestart) (Collision|BreakHitResult Hit))
  (if (!= OtherActor (Game|GetInstigator))
    (Effects|SpawnEmitteratLocation "/Game/MainFiles/P_Portal_Teleport_Exit.P_Portal_Teleport_Exit" (Transformation|GetActorLocation) (Transformation|GetActorRotation))
    (bind _returnvalue (Game|Damage|ApplyPointDamage _hitactor 1.0 _tracestart Hit 0 (Game|GetInstigator)))
    (Actor|DestroyActor)))

(event EventBeginPlay
  (Collision|IgnoreActorwhenMoving (Variables|Default|GetSphereComp) (Game|GetInstigator) true)
  (Audio|PlaySoundatLocation "/Game/MainFiles/SFX/ProtagProjectile/SFX_MagicProjectilePlayer.SFX_MagicProjectilePlayer" (Transformation|GetActorLocation) "0, 0, 0" 1.0 1.0 0.0 0 0 0 0))

(fn ConstructionScript)