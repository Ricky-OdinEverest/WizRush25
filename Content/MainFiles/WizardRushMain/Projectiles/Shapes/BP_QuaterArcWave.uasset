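; BP_QuaterArcWave is a projectile shape actor that detects hits in a forward-facing quarter-ring arc, currently as a debug prototype.
; A Delay on Tick spaces out multi radial sector traces from the actor origin with a 45-degree half angle.
; Distances to the CircInnerEdge and CircOuterEdge components set the ring radii.
; Hits are only printed, traces are debug-drawn, and an alternative CheckRadialSector call is left unconnected.
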(event EventBeginPlay)

(event Collision|EventActorBeginOverlap
  (params (OtherActor :type Actor%20Object%20Reference)))

(event EventTick
  (params (DeltaSeconds :type Float%20%28single-precision%29))
  (Utilities|FlowControl|Delay 2.0)
  (bind _outhits (Class|CollisionLibrary|RadialSectorTraceMulti (Transformation|GetActorLocation) (Math|Rotator|MakeRotfromX (Transformation|GetActorForwardVector)) 45.0 (Math|Vector|Distance(Vector) (Transformation|GetActorLocation) (Transformation|GetWorldLocation (Variables|Default|GetCircInnerEdge))) (Math|Vector|Distance(Vector) (Transformation|GetWorldLocation (Variables|Default|GetCircOuterEdge)) (Transformation|GetActorLocation)) "TraceTypeQuery3" false 0 "ForDuration"))
  (for _array_element _outhits
    (Development|PrintString (Utilities|String|ToString(Boolean) (.bBlockingHit (Collision|BreakHitResult _array_element))))
    (Development|PrintString (Utilities|GetDisplayName (.HitActor (Collision|BreakHitResult _array_element))))))

(fn ConstructionScript)