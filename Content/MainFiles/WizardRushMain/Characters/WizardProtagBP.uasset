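; Player wizard character Blueprint that handles sprint, aimed projectile, melee combo, portal-style dash and shield block.
; Input events delegate to combat, dash and stats components, using state flags to keep actions mutually exclusive; damage resets combos, and zero health shows the death widget.
; Tick feeds motion-warp targets for melee wind-up and auto-close, and prints debug state.
; The P key toggles a puddle material-parameter timeline.
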(event OnZeroHealthDelegate(StatsComp)
  ;[0.08755 1 0] Player Health And Death
  (bind _returnvalue (UserInterface|CreateWidget "/Game/MainFiles/UI/WBP_Death.WBP_Death_C"))
  (UserInterface|Viewport|AddtoViewport _returnvalue 0)
  (Class|WProtagWizard|HandleDeath))

(event OnHealthPercentUpdateDelegate(StatsComp)
  (params (Percentage :type Float%20%28single-precision%29))
  ;[0.08755 1 0] Player Health And Death
)

(event OnComponentHit(CapsuleComponent)
  (params (HitComponent :type Primitive%20Component%20Object%20Reference) (OtherActor :type Actor%20Object%20Reference) (OtherComp :type Primitive%20Component%20Object%20Reference) (NormalImpulse :type Vector :default "0, 0, 0") (Hit :type Hit%20Result%20Structure%20%28by%20ref%29)))

(event Custom|SetWarpTarget
  ;[0.991 1 0] Warp Target
)

(event Custom|Remove%20WarpTarget
  ;[0.991 1 0] Warp Target
  (Class|MotionWarpingComponent|RemoveAllWarpTargets (Variables|Default|GetPlayerMotionWarpingComponent)))

(event Custom|ResetActions
  (Variables|Default|SetIsSprinting false)
  (Variables|/Script/WizardRush.WDashComponent|SetbIsDashing (Variables|Default|GetDashComponent) false)
  (Variables|/Script/WizardRush.MeleeCombatComponent|SetbIsMeleeAttacking (Variables|Default|GetMeleeCombatComp) false)
  (Variables|Default|SetblockPlaying false)
  (Variables|/Script/WizardRush.WProjectileCombatComponent|SetbIsAiming (Variables|Default|GetProjectileCombatComp) false)
  (Development|SetHiddeninGame (Variables|Default|GetDashTrailGideonLarge) true false))

(event Custom|BlockActions)

(event Custom|GetUp
  (Effects|SpawnEmitteratLocation "/Game/MainFiles/P_Portal_Teleport_Exit.P_Portal_Teleport_Exit" (Transformation|GetActorLocation) "0, 0, 0" "3.000000,3.000000,3.000000")
  (Transformation|Teleport (.Location (Math|Transform|BreakTransform (Transformation|GetActorTransform))) (Variables|Default|GetPreDamageRotation))
  (Animation|PlayAnimMontage "/Game/MainFiles/PostTeleport.PostTeleport" 1.0 "None"))

(event Input|EnhancedActionEvents|EnhancedInputActionIA_Lockon
  (params (ActionValue :type Boolean) (ElapsedSeconds :type Float%20%28double-precision%29) (TriggeredSeconds :type Float%20%28double-precision%29) (InputAction :type Input%20Action%20Object%20Reference :default "/Game/MainFiles/WizardRushMain/Characters/Input/Actions/IA_Lockon.IA_Lockon"))
  ;[1 0 0] Melee Attacks. Will See How easy it is to updtae to just use motion warpong and anim Montages
)

(event Input|EnhancedActionEvents|EnhancedInputActionIA_MeleeAttack
  (params (ActionValue :type Boolean) (ElapsedSeconds :type Float%20%28double-precision%29) (TriggeredSeconds :type Float%20%28double-precision%29) (InputAction :type Input%20Action%20Object%20Reference :default "/Game/MainFiles/WizardRushMain/Characters/Input/Actions/IA_MeleeAttack.IA_MeleeAttack"))
  ;[1 0 0] Melee Attacks. Will See How easy it is to updtae to just use motion warpong and anim Montages
  (if (Math|Boolean|ANDBoolean (not (Variables|/Script/WizardRush.WDashComponent|GetbIsDashing (Variables|Default|GetDashComponent))) (not (Variables|/Script/WizardRush.WProjectileCombatComponent|GetbIsAiming (Variables|Default|GetProjectileCombatComp))) (not (Variables|/Script/WizardRush.MeleeCombatComponent|GetbIsMeleeAttacking (Variables|Default|GetMeleeCombatComp))) (not (Variables|Default|GetIsSprinting)) (not (Variables|Default|GetbPostHitInvincible)))
    (Class|MeleeCombatComponent|ComboAttack (Variables|Default|GetMeleeCombatComp))))

(event Input|EnhancedActionEvents|EnhancedInputActionIA_Sprint
  (params (ActionValue :type Boolean) (ElapsedSeconds :type Float%20%28double-precision%29) (TriggeredSeconds :type Float%20%28double-precision%29) (InputAction :type Input%20Action%20Object%20Reference :default "/Game/MainFiles/WizardRushMain/Characters/Input/Actions/IA_Sprint.IA_Sprint"))
  ;[1 0 0] Sprint Currently
  (:Started
    (if (Math|Boolean|ANDBoolean (not (Variables|/Script/WizardRush.WDashComponent|GetbIsDashing (Variables|Default|GetDashComponent))) (not (Variables|/Script/WizardRush.WProjectileCombatComponent|GetbIsAiming (Variables|Default|GetProjectileCombatComp))) (not (Variables|/Script/WizardRush.MeleeCombatComponent|GetbIsMeleeAttacking (Variables|Default|GetMeleeCombatComp))) (not (Variables|/Script/WizardRush.MeleeCombatComponent|GetbIsMeleeAttacking (Variables|Default|GetMeleeCombatComp))) (not (Variables|Default|GetbPostHitInvincible)))
      (Variables|Default|SetIsSprinting true)
      (Class|WProtagWizard|SprintStart)
      (else
        (Class|WProtagWizard|SprintStop :!label _label))))
  (:Completed
    (Variables|Default|SetIsSprinting false)
    (goto _label)))

(event Input|EnhancedActionEvents|EnhancedInputActionIA_OBJPrimary
  (params (ActionValue :type Boolean) (ElapsedSeconds :type Float%20%28double-precision%29) (TriggeredSeconds :type Float%20%28double-precision%29) (InputAction :type Input%20Action%20Object%20Reference :default "/Game/MainFiles/WizardRushMain/Characters/Input/Actions/IA_OBJPrimary.IA_OBJPrimary"))
  ;[1 0 0] Sprint Currently
  (:Started
    (Class|WProtagWizard|PrimaryAttackStart))
  (:Completed
    (Class|WProtagWizard|PrimaryAttackStop)))

(event Input|EnhancedActionEvents|EnhancedInputActionIA_Block
  (params (ActionValue :type Boolean) (ElapsedSeconds :type Float%20%28double-precision%29) (TriggeredSeconds :type Float%20%28double-precision%29) (InputAction :type Input%20Action%20Object%20Reference :default "/Game/MainFiles/WizardRushMain/Characters/Input/Actions/IA_Block.IA_Block"))
  ;[1 0 0] Block Ability
  (:Started
    (if (Math|Boolean|ANDBoolean (not (Variables|/Script/WizardRush.WDashComponent|GetbIsDashing (Variables|Default|GetDashComponent))) (not (Variables|/Script/WizardRush.WProjectileCombatComponent|GetbIsAiming (Variables|Default|GetProjectileCombatComp))) (not (Variables|/Script/WizardRush.MeleeCombatComponent|GetbIsMeleeAttacking (Variables|Default|GetMeleeCombatComp))) (not (Variables|Default|GetIsSprinting)) (not (Variables|Default|GetblockPlaying)) (not (Variables|Default|GetbPostHitInvincible)))
      (Variables|Default|SetblockPlaying true)
      (Collision|SetCollisionEnabled (Variables|Default|GetShieldCollisionSphere) "QueryAndPhysics")
      (Utilities|FlowControl|Sequence
        (:then_0
          (bind _returnvalue (Animation|PlayAnimMontage "/Game/MainFiles/AM_Wid_Block.AM_Wid_Block" 1.0 "None"))
          (Utilities|FlowControl|Delay _returnvalue)
          (Utilities|FlowControl|Sequence
            (:then_0
              (Variables|Default|SetblockPlaying false))
            (:then_1
              (Collision|SetCollisionEnabled (Variables|Default|GetShieldCollisionSphere) "NoCollision"))))
        (:then_1
          (Utilities|FlowControl|Delay 0.7)
          (for _array_element (Variables|Default|GetShield%20Hit)
            (if (Utilities|IsValid _array_element)
              (Components|DestroyComponent _array_element))))))))

(event EventBeginPlay
  (bind _actioncomp (Variables|Default|GetActionComp))
  ;[1 1 1] Initialize Controller
  (bind _asplayer_controller (Utilities|Casting|CastToPlayerController (Pawn|GetController)))
  (Input|AddMappingContext (PlayerController|LocalPlayerSubsystems|GetEnhancedInputLocalPlayerSubsystem _asplayer_controller) "/Game/MainFiles/WizardRushMain/Characters/Input/IMC_default.IMC_default" 0 "(bIgnoreAllPressedKeysUntilRelease=True,bForceImmediately=False,bNotifyUserSettings=False)")
  (Class|WActionComponent|AddAction _actioncomp "/Game/Actions/Action_Sprint.Action_Sprint_C")
  (Class|WActionComponent|AddAction _actioncomp "/Game/Actions/Action_ProjectileAttack.Action_ProjectileAttack_C"))

(event EventTick
  (params (DeltaSeconds :type Float%20%28single-precision%29))
  (Utilities|FlowControl|Sequence
    (:then_0
      ;[0.991 1 0] Warp Target
      (if (Variables|/Script/WizardRush.MeleeCombatComponent|GetbIsWindingUp (Variables|Default|GetMeleeCombatComp))
        (Class|MotionWarpingComponent|AddorUpdateWarpTargetfromLocationandRotation (Variables|Default|GetPlayerMotionWarpingComponent) "LookTarget" (Transformation|GetActorLocation self) (.ReturnValue (Class|WProtagWizard|GetMeleeRotationWarpTarget (Class|CharacterMovementComponent|GetLastUpdateRotation (Variables|Character|GetCharacterMovement)) DeltaSeconds)))
        (else
          (Variables|/Script/WizardRush.MeleeAutoCloseComponent|GetCurrentTargetActor (Variables|Default|GetMeleeAutoCloseComp)
            (:then
              (bind _returnvalue (Class|MeleeAutoCloseComponent|GetTranslationWarpTarget (Variables|Default|GetMeleeAutoCloseComp)))
              (Class|MotionWarpingComponent|AddorUpdateWarpTargetfromLocation (Variables|Default|GetPlayerMotionWarpingComponent) "TranslationTarget" _returnvalue)
              (bind _returnvalue_2 (Class|MeleeAutoCloseComponent|GetRotationWarpTarget (Variables|Default|GetMeleeAutoCloseComp)))
              (Class|MotionWarpingComponent|AddorUpdateWarpTargetfromLocation (Variables|Default|GetPlayerMotionWarpingComponent) "RotationTarget" _returnvalue_2))
            (:else)))))
    (:then_1
      (Development|PrintString (Utilities|String|Append "Dashing:" (Utilities|String|ToString(Boolean) (Variables|/Script/WizardRush.WDashComponent|GetbIsDashing (Variables|Default|GetDashComponent)))) true true "(R=0.000000,G=0.660000,B=1.000000,A=1.000000)" 2.0 "Dash")
      (Development|PrintString (Utilities|String|Append "Aiming:" (Utilities|String|ToString(Boolean) (Variables|/Script/WizardRush.WProjectileCombatComponent|GetbIsAiming (Variables|Default|GetProjectileCombatComp)))) true true "(R=0.000000,G=0.660000,B=1.000000,A=1.000000)" 2.0 "Aim")
      (Development|PrintString (Utilities|String|Append "Invincible:" (Utilities|String|ToString(Boolean) (Variables|Default|GetbPostHitInvincible))) true true "(R=0.000000,G=0.660000,B=1.000000,A=1.000000)" 2.0 "Invincible")
      (Development|PrintString (Utilities|String|Append "Sprinting" (Utilities|String|ToString(Boolean) (Variables|Default|GetIsSprinting))) true true "(R=0.000000,G=0.660000,B=1.000000,A=1.000000)" 2.0 "Sprinting")
      (Development|PrintString (Utilities|String|Append "Melee  Attack: " (Utilities|String|ToString(Boolean) (Variables|/Script/WizardRush.MeleeCombatComponent|GetbIsMeleeAttacking (Variables|Default|GetMeleeCombatComp)))) true true "(R=0.000000,G=0.660000,B=1.000000,A=1.000000)" 2.0 "Melee  Attack: "))))

(event Game|Damage|EventAnyDamage
  (params (Damage :type Float%20%28single-precision%29) (DamageType :type Damage%20Type%20Object%20Reference) (InstigatedBy :type Controller%20Object%20Reference) (DamageCauser :type Actor%20Object%20Reference))
  ;[0.08755 1 0] Player Health And Death
  (Variables|Default|SetPreDamageRotation (Variables|/Script/Engine.SceneComponent|GetRelativeRotation (Variables|Character|GetMesh)))
  (Class|StatsComponent|ReduceHealth (Variables|Default|GetStatsComp) Damage)
  (Class|WProtagWizard|PlayHurtAnim)
  (Class|MeleeCombatComponent|HandleResetCombo (Variables|Default|GetMeleeCombatComp)))

(event EventSendImpact
  (params (InHit :type Hit%20Result%20Structure%20%28by%20ref%29))
  (bind (_bblockinghit _binitialoverlap _time _distance _location _impactpoint _normal _impactnormal _physmat _hitactor _hitcomponent) (Collision|BreakHitResult InHit))
  ;[1 0 0] Block Ability
  (if (== _hitcomponent (Variables|Default|GetShieldCollisionSphere))
    (bind _returnvalue (Niagara|SpawnSystematLocation "/Game/Shooter_VFXPack/Particles/Update_1_1/P_LaserHit_ElectricityPurple.P_LaserHit_ElectricityPurple" _location (Math|Rotator|MakeRotfromX _impactnormal) "50.000000,50.000000,50.000000"))
    (Utilities|Array|Add (Variables|Default|GetShield%20Hit) _returnvalue)))

(event Input|ActionEvents|InputActionAim
  (params (Key :type Key%20Structure :default "None"))
  (bind _issprinting (Variables|Default|GetIsSprinting))
  (bind _projectilecombatcomp (Variables|Default|GetProjectileCombatComp))
  (bind _meleecombatcomp (Variables|Default|GetMeleeCombatComp))
  (bind _bposthitinvincible (Variables|Default|GetbPostHitInvincible))
  (bind _dashcomponent (Variables|Default|GetDashComponent))
  (bind _bismeleeattacking (Variables|/Script/WizardRush.MeleeCombatComponent|GetbIsMeleeAttacking _meleecombatcomp))
  (bind _bisdashing (Variables|/Script/WizardRush.WDashComponent|GetbIsDashing _dashcomponent))
  (bind _returnvalue (Math|Boolean|ORBoolean _bisdashing _bismeleeattacking _issprinting _bposthitinvincible))
  ;[1 0 0] Aim And Shoot. /// Should Update to Enhanced IA
  (:Pressed
    (if (not _returnvalue)
      (Class|WProjectileCombatComponent|StartAiming _projectilecombatcomp)
      (Animation|PlayAnimMontage "/Game/MainFiles/GidToWidPrimary_Attack_A_Medium_Montage.GidToWidPrimary_Attack_A_Medium_Montage" 0.5 "Start")
      (Utilities|FlowControl|Delay 0.2)
      (if (Variables|/Script/WizardRush.WProjectileCombatComponent|GetbIsAiming (Variables|Default|GetProjectileCombatComp))
        (Animation|PlayAnimMontage "/Game/MainFiles/GidToWidPrimary_Attack_A_Medium_Montage.GidToWidPrimary_Attack_A_Medium_Montage" 0.2 "Loop"))))
  (:Released
    (if (not _returnvalue)
      (Class|WProjectileCombatComponent|StopAiming _projectilecombatcomp)
      (Animation|PlayAnimMontage "/Game/MainFiles/GidToWidPrimary_Attack_A_Medium_Montage.GidToWidPrimary_Attack_A_Medium_Montage" 1.0 "end"))))

(event Input|ActionEvents|InputActionDashCharge
  (params (Key :type Key%20Structure :default "None"))
  (bind _projectilecombatcomp (Variables|Default|GetProjectileCombatComp))
  (bind _issprinting (Variables|Default|GetIsSprinting))
  (bind _bposthitinvincible (Variables|Default|GetbPostHitInvincible))
  (bind _dashcomponent (Variables|Default|GetDashComponent))
  (bind _returnvalue (not _issprinting))
  (bind _returnvalue_2 (not _bposthitinvincible))
  (bind _bisaiming (Variables|/Script/WizardRush.WProjectileCombatComponent|GetbIsAiming _projectilecombatcomp))
  (bind _returnvalue_3 (not _bisaiming))
  (bind _returnvalue_4 (Math|Boolean|ANDBoolean _returnvalue _returnvalue_3 _returnvalue_2))
  ;[1 0 0] Dash Mechanic // Ensure Teleport Does not sweep or collide with objects
  (:Pressed
    (if _returnvalue_4
      (Class|WDashComponent|DashCharge _dashcomponent)
      (if (Math|Boolean|ANDBoolean (Variables|/Script/WizardRush.WDashComponent|GetbIsDashing (Variables|Default|GetDashComponent)) (not (Variables|/Script/WizardRush.MeleeCombatComponent|GetbIsMeleeAttacking (Variables|Default|GetMeleeCombatComp))) (not (Variables|/Script/WizardRush.WProjectileCombatComponent|GetbIsAiming (Variables|Default|GetProjectileCombatComp))) (not (Variables|Default|GetIsSprinting)) (not (Variables|Default|GetbPostHitInvincible)))
        (Components|Animation|PlayAnimation (Variables|Character|GetMesh) "/Game/MainFiles/EpicCharacter_Interact.EpicCharacter_Interact" true)
        (Effects|SpawnEmitteratLocation "/Game/MainFiles/P_Portal_Cast.P_Portal_Cast" (Transformation|GetActorLocation) "0, 0, 0" "2.000000,2.000000,2.000000")
        (Development|SetHiddeninGame (Variables|Default|GetDashTrailGideonLarge) false false)
        (else
          (Components|Animation|SetAnimationMode (Variables|Character|GetMesh) "AnimationBlueprint" true :!label _label)
          (Utilities|FlowControl|Delay 0.2)
          (Development|SetHiddeninGame (Variables|Default|GetDashTrailGideonLarge) true false)))))
  (:Released
    (if _returnvalue_4
      (Class|WDashComponent|DashInitiate _dashcomponent)
      (Effects|SpawnEmitteratLocation "/Game/MainFiles/P_Portal_Teleport_Exit.P_Portal_Teleport_Exit" (Transformation|GetActorLocation) "0, 0, 0" "3.000000,3.000000,3.000000")
      (goto _label))))

(event Input|KeyboardEvents|T
  (params (Key :type Key%20Structure :default "None")))

(event Input|KeyboardEvents|P
  (params (Key :type Key%20Structure :default "None"))
  ;[0 0.7221 1] Puddles
  (:Pressed
    (Utilities|FlowControl|FlipFlop
      (:A
        (bind _newtrack_0 (Timeline|Timeline Play)
          (:Update
            (Rendering|Material|SetScalarParameterValue "/Prismatiscape/Prismatiscape_MPC.Prismatiscape_MPC" "Puddles" _newtrack_0 :!class /Script/Engine.KismetMaterialLibrary))))
      (:B
        (Timeline|Timeline Reverse)))))

(fn ConstructionScript)