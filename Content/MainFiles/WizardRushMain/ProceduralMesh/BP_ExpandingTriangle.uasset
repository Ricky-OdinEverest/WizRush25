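; Procedural mesh actor that builds a triangle or subdivided vertical grid by enum, with the triangle expanding over time.
; Construction Script clears mesh data, runs the chosen draw function, then creates a section with collision.
; Grid generation derives UVs, indices, normals and tangents; the triangle sets only vertices and indices.
; Tick uses a Delay to step up triangle scale, hits only print, and DrawCylinder is never called.
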(event OnComponentHit(ProceduralMesh)
  (params (HitComponent :type Primitive%20Component%20Object%20Reference) (OtherActor :type Actor%20Object%20Reference) (OtherComp :type Primitive%20Component%20Object%20Reference) (NormalImpulse :type Vector :default "0, 0, 0") (Hit :type Hit%20Result%20Structure%20%28by%20ref%29))
  (Development|PrintString "Hit Occured"))

(event Custom|Clear%20Mesh%20Data
  (Utilities|Array|Clear (Variables|Default|GetVertex))
  (Utilities|Array|Clear (Variables|Default|GetTriangle))
  (Utilities|Array|Clear (Variables|Default|GetUV)))

(event EventBeginPlay)

(event Collision|EventActorBeginOverlap
  (params (OtherActor :type Actor%20Object%20Reference)))

(event EventTick
  (params (DeltaSeconds :type Float%20%28single-precision%29))
  (bind _proceduralmesh (Variables|Default|GetProceduralMesh))
  (if (Utilities|Enum|Equal(Enum) (Variables|Default|GetEnum) "NewEnumerator0")
    (Utilities|FlowControl|Delay 0.2)
    (Transformation|SetRelativeScale3D _proceduralmesh (+ (Variables|/Script/Engine.SceneComponent|GetRelativeScale3D _proceduralmesh) "1.000000,0.500000,0.500000"))))

(fn ConstructionScript
  (CallFunction|ClearMeshData)
  (Utilities|FlowControl|Sequence
    (:then_0
      ;[1 1 1] MakeData
      (switch Utilities|FlowControl|Switch|SwitchonE_ShapeType (Variables|Default|GetEnum)
        (:NewEnumerator0
          (CallFunction|DrawTriangle))
        (:NewEnumerator1
          (CallFunction|DrawQuad))))
    (:then_1
      ;[1 1 1] CalculateNormals
      (Class|ProceduralMeshComponent|CreateMeshSectionLinearColor (Variables|Default|GetProceduralMesh) 0 (Variables|Default|GetVertex) (Variables|Default|GetTriangle) (Variables|Default|GetNormals) (Variables|Default|GetUV) 0 0 0 0 (Variables|Default|GetTangents) true true))))

(fn DrawQuad
  ;[1 1 1] X & Y Index
  (for _index (range 0 (LocalVariables|GetXLength))
    (LocalVariables|SetX _index)
    (for _index_2 (range 0 (LocalVariables|GetYLength))
      (LocalVariables|SetY _index_2)
      (Utilities|FlowControl|Sequence
        (:then_0
          ;[1 1 1] MakeVertexLocations
          (Utilities|Array|Add (Variables|Default|GetVertex) (Math|Vector|MakeVector (* (LocalVariables|GetX) 5e+01) 0.0 (* (LocalVariables|GetY) 5e+01))))
        (:then_1
          ;[1 1 1] Make UV Locations
          (Utilities|Array|Add (Variables|Default|GetUV) (Math|Vector2D|MakeVector2D (/ (Math|Conversions|ToFloat(Integer) (LocalVariables|GetX)) (Math|Conversions|ToFloat(Integer) (LocalVariables|GetXLength))) (/ (Math|Conversions|ToFloat(Integer) (LocalVariables|GetY)) (Math|Conversions|ToFloat(Integer) (LocalVariables|GetYLength)))))))))
  (Utilities|FlowControl|Sequence
    (:then_0
      ;[1 1 1] CreateTriangles
      (bind _triangles (Class|KismetProceduralMeshLibrary|CreateGridMeshTriangles (+ (LocalVariables|GetXLength) 1) (+ (LocalVariables|GetYLength) 1) true))
      (Variables|Default|SetTriangle _triangles))
    (:then_1
      ;[1 1 1] Tangents and Normals For Mesh
      (bind (_normals _tangents) (Class|KismetProceduralMeshLibrary|CalculateTangentsforMesh (Variables|Default|GetVertex) (Variables|Default|GetTriangle) (Variables|Default|GetUV)))
      (Variables|Default|SetNormals _normals)
      (Variables|Default|SetTangents _tangents))))

(fn DrawTriangle
  (Variables|Default|SetVertex (Utilities|Array|MakeArray "100.000000,100.000000,0.000000" "0.000000,-0.000000,0.000000" "100.000000,-100.000000,0.000000"))
  (Variables|Default|SetTriangle (Utilities|Array|MakeArray 2 1 0)))

(fn DrawCylinder
  ;[1 1 1] X & Y Index
  (for _index (range 0 (LocalVariables|GetZLength))
    (LocalVariables|SetZ _index)
    (for _index_2 (range 0 (LocalVariables|GetXLength))
      (LocalVariables|SetX _index_2)
      (Utilities|FlowControl|Sequence
        (:then_0
          ;[1 1 1] MakeVertexLocations
          (Utilities|Array|Add (Variables|Default|GetVertex) (+ (* (Math|Vector|RotateVectorAroundAxis (Transformation|GetActorForwardVector) (* (/ (Math|Conversions|ToFloat(Integer) (LocalVariables|GetX)) (Math|Conversions|ToFloat(Integer) (LocalVariables|GetXLength))) 3.6e+02) (Transformation|GetActorUpVector)) 1e+02) (Math|Vector|MakeVector 0.0 0.0 (* (LocalVariables|GetZ) 5e+01)))))
        (:then_1
          ;[1 1 1] Make UV Locations
          (Utilities|Array|Add (Variables|Default|GetUV) (Math|Vector2D|MakeVector2D (/ (Math|Conversions|ToFloat(Integer) (LocalVariables|GetZ)) (Math|Conversions|ToFloat(Integer) (LocalVariables|GetZLength))) (/ (Math|Conversions|ToFloat(Integer) (LocalVariables|GetX)) (Math|Conversions|ToFloat(Integer) (LocalVariables|GetXLength)))))))))
  (Utilities|FlowControl|Sequence
    (:then_0
      ;[1 1 1] CreateTriangles
      (bind _triangles (Class|KismetProceduralMeshLibrary|CreateGridMeshTriangles (+ (LocalVariables|GetZ) 1) (+ (LocalVariables|GetXLength) 1) true))
      (Variables|Default|SetTriangle _triangles))
    (:then_1
      ;[1 1 1] Tangents and Normals For Mesh
      (bind (_normals _tangents) (Class|KismetProceduralMeshLibrary|CalculateTangentsforMesh (Variables|Default|GetVertex) (Variables|Default|GetTriangle) (Variables|Default|GetUV)))
      (Variables|Default|SetNormals _normals)
      (Variables|Default|SetTangents _tangents))))