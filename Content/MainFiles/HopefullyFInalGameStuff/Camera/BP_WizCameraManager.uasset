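; Player camera manager for the wizard protagonist that frames the player together with a boss target.
; BeginPlay looks once for pawns tagged CamTarget, and Tick tracks the player's distance to the first one found.
; BlueprintUpdateCamera keeps the player camera's rotation and FOV, placing the view behind the pair's midpoint by that distance, with a minimum pullback.
; Without a target, it uses the player camera's own location.
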(event EventBeginPlay
  (bind _outactors (Actor|GetAllActorsOfClasswithTag "/Script/Engine.Pawn" "CamTarget"))
  (Variables|Default|SetCamTarget _outactors)
  (bind _output_get (Variables|Default|SetBossTargetFound (> (Utilities|Array|Length (Variables|Default|GetCamTarget)) 0))))

(event Collision|EventActorBeginOverlap
  (params (OtherActor :type Actor%20Object%20Reference)))

(event EventTick
  (params (DeltaSeconds :type Float%20%28single-precision%29))
  (if (Variables|Default|GetBossTargetFound)
    (Variables|Default|SetDistanceBetweenActors (Transformation|GetDistanceTo (Pawn|GetControlledPawn (Game|Player|GetOwningPlayerController)) (Utilities|Array|Get(acopy) (Variables|Default|GetCamTarget))))))

(fn ConstructionScript)

(fn BlueprintUpdateCamera
  (params (CameraTarget :type Actor%20Object%20Reference))
  (bind _distancebetweenactors (Variables|Default|GetDistanceBetweenActors))
  (bind _aswizard_protag_bp (Utilities|Casting|CastToWizardProtagBP CameraTarget))
  (bind _output_get (LocalVariables|SetPlayer _aswizard_protag_bp))
  (LocalVariables|SetCamFov (Variables|/Script/Engine.CameraComponent|GetFieldOfView (Variables|/Script/WizardRush.WProtagWizard|GetCameraComp _output_get)))
  (bind _output_get_2 (Variables|Default|SetCamInitialRotation (.Rotation (Math|Transform|BreakTransform (Transformation|GetWorldTransform (Variables|/Script/WizardRush.WProtagWizard|GetCameraComp _output_get))))))
  (LocalVariables|SetCaminitialLocation (.Location (Math|Transform|BreakTransform (Transformation|GetWorldTransform (Variables|/Script/WizardRush.WProtagWizard|GetCameraComp _output_get)))))
  (if (Variables|Default|GetBossTargetFound)
    (LocalVariables|SetMidpoint (/ (+ (Transformation|GetActorLocation (Utilities|Array|Get(acopy) (Variables|Default|GetCamTarget))) (Transformation|GetActorLocation (LocalVariables|GetPlayer))) 2.0))
    (LocalVariables|SetNewLocation (+ (* (Math|Vector|GetForwardVector _output_get_2) (* (Math|Float|Clamp(Float) _distancebetweenactors 8e+02 _distancebetweenactors) -1.0)) (LocalVariables|GetMidpoint)))
    (else
      (LocalVariables|SetNewLocation (.Location (Math|Transform|BreakTransform (Transformation|GetWorldTransform (Variables|/Script/WizardRush.WProtagWizard|GetCameraComp _output_get)))))))
  (return (LocalVariables|GetNewLocation) (Variables|Default|GetCamInitialRotation) (LocalVariables|GetCamFov) true))