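; BP_TriangleWave is a triangle-shaped attack wave that faces along its instigator's forward vector and damages what it reaches.
; Each Tick grows the mesh by a fixed, frame-rate-dependent step up to a scale cap, then optionally self-destructs after a delay.
; A per-frame cone trace, sized from marker component positions, applies point damage and adds hit actors to an ignore list so each is damaged only once.
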(event Custom|GrowShape
  (bind _output_get (Variables|Default|SetCurrScale (+ (Variables|Default|GetCurrScale) (* (Variables|Default|GetScaleGrowthVector) (Variables|Default|GetScaleGrowthRate)))))
  (if (<= (.x (Variables|Default|GetCurrScale)) (* (Variables|Default|GetScaleGrowthCap) (.X (Math|Vector|BreakVector (Variables|Default|GetInitialScale)))))
    (Transformation|SetRelativeScale3D (Variables|Default|GetCustTraingleMesh) _output_get)
    (elif (Variables|Default|GetDestroyAfterFullSize)
      (CallFunction|SelfDestruct))))

(event Custom|SelfDestruct
  (Utilities|FlowControl|Delay (Variables|Default|GetSelfDestructDelay))
  (Actor|DestroyActor))

(event EventBeginPlay
  (Variables|Default|SetPlayer (Game|Player|GetPlayerPawn 0))
  (Transformation|SetRelativeScale3D (Variables|Default|GetCustTraingleMesh) (Variables|Default|GetInitialScale))
  (Variables|Default|SetCurrScale (Variables|Default|GetInitialScale))
  (Transformation|SetActorRotation self (Math|Conversions|RotationFromXVector (Transformation|GetActorForwardVector (Game|GetInstigator))) true))

(event Collision|EventActorBeginOverlap
  (params (OtherActor :type Actor%20Object%20Reference)))

(event EventTick
  (params (DeltaSeconds :type Float%20%28single-precision%29))
  (bind (_returnvalue _returnvalue2 _returnvalue3 _returnvalue4) (CallFunction|GetTraceVariables))
  (Utilities|FlowControl|Sequence
    (:then_0
      (bind (_outhits _returnvalue_2) (Class|CollisionLibrary|ConeTraceMulti _returnvalue _returnvalue2 _returnvalue3 _returnvalue4 0.0 "TraceTypeQuery3" false (Variables|Default|GetActors%20to%20Ignore) "None" "(R=0.000000,G=1.000000,B=1.000000,A=1.000000)" "(R=1.000000,G=0.000000,B=0.126577,A=1.000000)"))
      (if _returnvalue_2
        (for _array_element _outhits
          (Utilities|Array|AddUnique (Variables|Default|GetActors%20to%20Ignore) (.HitActor (Collision|BreakHitResult _array_element)))
          (Utilities|Array|AddUnique (Variables|Default|GetHitActors) _array_element)
          (Game|Damage|ApplyPointDamage (.HitActor (Collision|BreakHitResult _array_element)) 1.0 (.Location (Collision|BreakHitResult _array_element)) _array_element 0 (Game|GetInstigator)))))
    (:then_1
      (CallFunction|GrowShape))))

(fn ConstructionScript
  (bind _output_get (Variables|Default|SetInitialFacingDirection (Transformation|GetActorForwardVector (Game|GetInstigator)))))

(fn GetHalfAngle
  (return (Math|Trig|RadiansToDegrees (Math|Trig|Atan(Degrees) (/ (* (Math|Vector|Distance(Vector) (Transformation|GetWorldLocation (Variables|Default|GetCircPoint1)) (Transformation|GetWorldLocation (Variables|Default|GetCircPoint2))) 0.5) (Math|Vector|Distance(Vector) (Transformation|GetWorldLocation (Variables|Default|GetTraceStart)) (* (+ (Transformation|GetWorldLocation (Variables|Default|GetCircPoint1)) (Transformation|GetWorldLocation (Variables|Default|GetCircPoint2))) 0.5)))))))

(fn GetTraceVariables
  (bind _tracestart (Variables|Default|GetTraceStart))
  (bind _returnvalue (Transformation|GetWorldLocation _tracestart))
  (return _returnvalue (Math|Rotator|MakeRotfromX (Transformation|GetActorForwardVector self)) (Math|Vector|Distance(Vector) _returnvalue (Transformation|GetWorldLocation (Variables|Default|GetTraceEnd))) (CallFunction|GetHalfAngle)))