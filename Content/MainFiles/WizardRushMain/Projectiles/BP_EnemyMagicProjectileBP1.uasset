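; BP_EnemyMagicProjectileBP1 is an enemy magic projectile that bursts on impact.
; On BeginPlay, its sphere collision component ignores the instigator during movement.
; When the sphere hits anything other than the instigator, it spawns a portal teleport exit particle effect at the projectile's transform and destroys the actor.
; The graph itself applies no damage.
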(event OnComponentHit(SphereComp)
  (params (HitComponent :type Primitive%20Component%20Object%20Reference) (OtherActor :type Actor%20Object%20Reference) (OtherComp :type Primitive%20Component%20Object%20Reference) (NormalImpulse :type Vector :default "0, 0, 0") (Hit :type Hit%20Result%20Structure%20%28by%20ref%29))
  (if (!= OtherActor (Game|GetInstigator))
    (Effects|SpawnEmitteratLocation "/Game/MainFiles/P_Portal_Teleport_Exit.P_Portal_Teleport_Exit" (Transformation|GetActorLocation) (Transformation|GetActorRotation))
    (Actor|DestroyActor)))

(event EventBeginPlay
  (Collision|IgnoreActorwhenMoving (Variables|Default|GetSphereComp) (Game|GetInstigator) true))

(fn ConstructionScript)